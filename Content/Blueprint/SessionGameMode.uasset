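; Lobby game mode for an online session that tracks connected players and launches the match map via server travel.
; On server PostLogin it stores the controller, reads session settings from SessionGameInstance, sets up the SessionPC lobby and spawns a character at the first PlayerStart.
; Respawns and logouts trigger EveryoneUpdate, which pushes player counts and statuses to every SessionPC.
; AddToKickList is an empty stub, and CanWeStart turns true with any player present.
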(event Custom|EveryoneUpdate
  (bind _allplayercontrollers (Variables|ServerSettings|GetAllPlayerControllers))
  (bind _output_get (Variables|ServerSettings|SetCurrentNumOfPlayers (Utilities|Array|Length (Variables|ServerSettings|GetAllPlayerControllers))))
  (if (> _output_get 0)
    (Utilities|Array|Clear (Variables|ServerSettings|GetConnectedPlayerStatus))
    (for _array_element _allplayercontrollers
      (bind _assession_pc (Utilities|Casting|CastToSessionPC _array_element))
      (Utilities|Array|Add (Variables|ServerSettings|GetConnectedPlayerStatus) (Variables|/OnlineSessionSystem/Blueprint/SessionPC.SessionPC_C|GetPlayer%20Network%20Status _assession_pc))
      (Default|UpdateNumOfPlayers _assession_pc (Variables|ServerSettings|GetCurrentNumOfPlayers) (Variables|ServerSettings|GetNum%20Of%20Players)))
    (for _array_element_2 _allplayercontrollers
      (bind _assession_pc_2 (Utilities|Casting|CastToSessionPC _array_element_2))
      (Default|AddPlayerStatus _assession_pc_2 (Variables|ServerSettings|GetConnectedPlayerStatus))
      (CallFunction|AddtoKickList))
    (Variables|ServerSettings|SetCanWeStart true)))

(event Custom|LaunchGame
  (bind _returnvalue (Game|GetPlayerController 0))
  (Development|ExecuteConsoleCommand "servertravel /OnlineSessionSystem/Game/Level/ThirdPersonMap" _returnvalue)
  (Viewport|RemoveAllWidgets)
  (Input|SetInputModeGameOnly _returnvalue false))

(event Custom|RespawnPlayer
  (params (Controller :type Player%20Controller%20Object%20Reference))
  (bind _returnvalue (Pawn|GetControlledPawn Controller))
  (Utilities|IsValid _returnvalue
    (:Is%20Valid
      (Actor|DestroyActor _returnvalue))
    (:Is%20Not%20Valid
      _))
  (bind _returnvalue_2 (Game|SpawnActorfromClass "/OnlineSessionSystem/Game/Characters/Blueprints/BP_ThirdPersonCharacter.BP_ThirdPersonCharacter_C" (Transformation|GetActorTransform (Utilities|Array|Get(acopy) (Variables|ServerSettings|GetPlayerStarts))) "Undefined" 0 0))
  (Pawn|Possess Controller _returnvalue_2)
  (CallFunction|EveryoneUpdate))

(event Custom|AddToKickList)

(event EventBeginPlay)

(event EventOnLogout
  (params (ExitingController :type Controller%20Object%20Reference))
  (bind (_array_element _array_index) (Utilities|Array|ForEachLoopwithBreak (Variables|ServerSettings|GetAllPlayerControllers) :!label _label)
    (:LoopBody
      (if (== _array_element ExitingController)
        (goto _label Break)))
    (:Completed
      (Utilities|Array|RemoveIndex (Variables|ServerSettings|GetAllPlayerControllers) _array_index)
      (Utilities|Array|RemoveIndex (Variables|ServerSettings|GetConnectedPlayerStatus) _array_index)
      (CallFunction|EveryoneUpdate))))

(event EventPostLogin
  (params (NewPlayer :type Player%20Controller%20Object%20Reference))
  (Networking|SwitchHasAuthority
    (:Authority
      (Utilities|FlowControl|Sequence
        (:then_0
          (Utilities|Array|Add (Variables|ServerSettings|GetAllPlayerControllers) NewPlayer)
          (bind _assession_game_instance (Utilities|Casting|CastToSessionGameInstance (Game|GetGameInstance)))
          (Variables|ServerSettings|SetServer%20Name (Variables|/OnlineSessionSystem/Blueprint/SessionGameInstance.SessionGameInstance_C|GetServer%20Name _assession_game_instance))
          (Variables|ServerSettings|SetNum%20Of%20Players (Variables|/OnlineSessionSystem/Blueprint/SessionGameInstance.SessionGameInstance_C|GetNum%20Of%20Players _assession_game_instance))
          (bind _outactors (Actor|GetAllActorsOfClass "/Script/Engine.PlayerStart"))
          (Variables|ServerSettings|SetPlayerStarts _outactors))
        (:then_1
          (bind _assession_pc (Utilities|Casting|CastToSessionPC NewPlayer))
          (Default|SetupLobby _assession_pc)
          (Default|SetupLobbyMenu _assession_pc (Variables|ServerSettings|GetServer%20Name)))
        (:then_2
          (CallFunction|RespawnPlayer NewPlayer))))))

(fn ConstructionScript)