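; SessionGameInstance is a Game Instance Blueprint that manages front-end menus and multiplayer sessions.
; Show events add main, host, options, server and loading widgets to the viewport, reusing cached instances for all but the server menu.
; LaunchLobby shows loading, creates a LAN-optional session and opens Lobby as a listen server on success.
; It also joins and destroys sessions, and only prints network and travel errors.
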(event Custom|ShowMainMenu
  ;[1 1 1] Show Main Menu & Show Mouse Cursor
  (Utilities|IsValid (Variables|Widgets|GetMainMenu)
    (:Is%20Valid
      _)
    (:Is%20Not%20Valid
      (bind _returnvalue (UserInterface|CreateWidget "/OnlineSessionSystem/UI/MainMenu/WBP_MainMenu.WBP_MainMenu_C" (Game|GetPlayerController 0)))
      (Variables|Widgets|SetMainMenu _returnvalue)))
  (UserInterface|Viewport|AddtoViewport (Variables|Widgets|GetMainMenu) 0)
  (Variables|/Script/Engine.PlayerController|SetbShowMouseCursor (Game|GetPlayerController 0) true))

(event Custom|ShowHostMenu
  ;[1 1 1] Show Host Menu
  (Utilities|IsValid (Variables|Widgets|GetHostMenu)
    (:Is%20Valid
      _)
    (:Is%20Not%20Valid
      (bind _returnvalue (UserInterface|CreateWidget "/OnlineSessionSystem/UI/MainMenu/WBP_HostMenu.WBP_HostMenu_C" (Game|GetPlayerController 0)))
      (Variables|Widgets|SetHostMenu _returnvalue)))
  (UserInterface|Viewport|AddtoViewport (Variables|Widgets|GetHostMenu) 0))

(event Custom|ShowServerMenu
  ;[1 1 1] Show Server Menu - Add To Viewport when called
  (bind _returnvalue (UserInterface|CreateWidget "/OnlineSessionSystem/UI/MainMenu/WBP_ServerMenu.WBP_ServerMenu_C" (Game|GetPlayerController 0)))
  (UserInterface|Viewport|AddtoViewport _returnvalue 0))

(event Custom|ShowOptionMenu
  ;[1 1 1] Show Options Menu
  (Utilities|IsValid (Variables|Widgets|GetOptionsMenu)
    (:Is%20Valid
      _)
    (:Is%20Not%20Valid
      (bind _returnvalue (UserInterface|CreateWidget "/OnlineSessionSystem/UI/MainMenu/WBP_OptionsMenu.WBP_OptionsMenu_C" (Game|GetPlayerController 0)))
      (Variables|Widgets|SetOptionsMenu _returnvalue)))
  (UserInterface|Viewport|AddtoViewport (Variables|Widgets|GetOptionsMenu) 0)
  (Variables|/Script/Engine.PlayerController|SetbShowMouseCursor (Game|GetPlayerController 0) true))

(event Custom|LaunchLobby
  (params (NumOfPlayers :type Integer) (IsLan? :type Boolean) (ServerName :type Text))
  ;[1 1 1] Open Level When Success Create Session
  (Variables|Default|SetNum%20Of%20Players NumOfPlayers)
  (Variables|Default|SetServer%20Name ServerName)
  (CallFunction|ShowLoadingScreen)
  (|Session (Game|GetPlayerController 0) (Variables|Default|GetNum%20Of%20Players) IsLan?
    (:OnSuccess
      (Game|OpenLevel(byName) "Lobby" true "listen"))))

(event Custom|ShowLoadingScreen
  ;[1 1 1] Show Loading Screen
  (Utilities|IsValid (Variables|Widgets|GetLoadingScreen)
    (:Is%20Valid
      _)
    (:Is%20Not%20Valid
      (bind _returnvalue (UserInterface|CreateWidget "/OnlineSessionSystem/UI/Game/WBP_LoadingScreen.WBP_LoadingScreen_C" (Game|GetPlayerController 0)))
      (Variables|Widgets|SetLoadingScreen _returnvalue)))
  (UserInterface|Viewport|AddtoViewport (Variables|Widgets|GetLoadingScreen) 0))

(event Custom|JoinServer
  (params (SessionResult :type Blueprint%20Session%20Result%20Structure))
  ;[1 1 1] Join Server
  (CallFunction|ShowLoadingScreen)
  (|JoinSession (Game|GetPlayerController 0) SessionResult))

(event Custom|DestroySession
  (params (PlayerController :type Player%20Controller%20Object%20Reference))
  (|DestroySession PlayerController))

(event EventHandleNetworkError
  (params (FailureType :type ENetworkFailure%20Enum :default "NetDriverAlreadyExists") (bIsServer :type Boolean))
  (if bIsServer
    _
    (else
      _))
  (Development|PrintString (Utilities|String|EnumtoString FailureType)))

(event EventHandleTravelError
  (params (FailureType :type ETravelFailure%20Enum :default "NoLevel"))
  (Development|PrintString (Utilities|String|EnumtoString FailureType)))