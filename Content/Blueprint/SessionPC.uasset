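; SessionPC is a player controller that manages a player's side of a multiplayer session lobby.
; It creates the lobby menu and passes status changes to SessionGameMode by storing them and calling EveryoneUpdate.
; Other events refresh the player list and count or swap the menu for a loading screen.
; Being kicked opens MainMenu and destroys the session, which EndPlay also does.
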(event Custom|SetupLobby
  (CallFunction|UpdateLobby (Variables|Default|GetPlayer%20Network%20Status) false))

(event Custom|UpdateLobby
  (params (PlayerNetworkStatus :type Text) (IsChangedStatus :type Boolean))
  (Variables|Default|SetPlayer%20Network%20Status PlayerNetworkStatus)
  (bind _assession_game_mode (Utilities|Casting|CastToSessionGameMode (Game|GetGameMode)))
  (Default|EveryoneUpdate _assession_game_mode))

(event Custom|SetupLobbyMenu
  (params (Server%20Name :type Text))
  (Variables|Default|SetbShowMouseCursor true)
  (bind _returnvalue (UserInterface|CreateWidget "/OnlineSessionSystem/UI/Lobby/WBP_LobbyMenu.WBP_LobbyMenu_C" 0 Server%20Name))
  (bind _output_get (Variables|Default|SetLobbyMenu _returnvalue))
  (UserInterface|Viewport|AddtoViewport _output_get 0)
  (Input|SetInputModeGameandUI self _output_get "DoNotLock" true false))

(event Custom|AddPlayerStatus
  (params (ConnectedPlayerStatus :type Array%20of%20Texts))
  (bind _lobbymenu (Variables|Default|GetLobbyMenu))
  (Variables|Default|SetAll%20Player%20Status ConnectedPlayerStatus)
  (Utilities|IsValid _lobbymenu
    (:Is%20Valid
      (Default|ClearPlayerList _lobbymenu)
      (for _array_element (Variables|Default|GetAll%20Player%20Status)
        (Default|UpdatePlayerWindow (Variables|Default|GetLobbyMenu) _array_element)))))

(event Custom|ShowLoadingScreen
  (Widget|RemovefromParent (Variables|Default|GetLobbyMenu))
  (bind _returnvalue (UserInterface|CreateWidget "/OnlineSessionSystem/UI/Game/WBP_LoadingScreen.WBP_LoadingScreen_C" self))
  (UserInterface|Viewport|AddtoViewport _returnvalue 0))

(event Custom|UpdateNumOfPlayers
  (params (CurrentPlayerNum :type Integer) (MaxPlayerNum :type Integer))
  (bind _lobbymenu (Variables|Default|GetLobbyMenu))
  (Utilities|IsValid _lobbymenu
    (:Is%20Valid
      (Variables|/OnlineSessionSystem/UI/Lobby/WBP_LobbyMenu.WBP_LobbyMenu_C|SetNumOfPlayers _lobbymenu (Utilities|Text|FormatText "{CurrentNums} / {MaxNums}" (Utilities|Text|ToText(Integer) CurrentPlayerNum) (Utilities|Text|ToText(Integer) MaxPlayerNum))))))

(event Custom|Kicked
  (Game|OpenLevel(byName) "MainMenu")
  (|DestroySession self))

(event EventBeginPlay)

(event EventEndPlay
  (params (EndPlayReason :type EEndPlayReason%20Enum :default "Destroyed"))
  (|DestroySession self))

(fn ConstructionScript)